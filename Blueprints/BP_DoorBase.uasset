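; Base door Blueprint that swings open when any actor begins overlapping it and closes when an overlap ends.
; One timeline, played forward or in reverse, drives the DoorRotator's relative yaw up to MaxDoorOpenAngle.
; InProgress blocks open and close requests mid-swing without queuing them, and the timeline's direction on finish sets IsDoorOpen.
; Begin overlap also prints a test string.
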(event Custom|OpenDoor
  ;[1 1 1] Door opens and closes
  (if (not (Variables|Default|GetInProgress))
    (if (not (Variables|Default|GetIsDoorOpen))
      (bind (_direction _progressionopening) (Timeline|Timeline_0 PlayFromStart)
        (:Update
          (Variables|Default|SetInProgress true)
          (Transformation|SetRelativeRotation (Variables|Default|GetDoorRotator) (Math|Rotator|MakeRotator 0.0 0.0 (* (Variables|Default|GetMaxDoorOpenAngle) _progressionopening)) false false))
        (:Finished
          (Variables|Default|SetInProgress false)
          (switch Utilities|FlowControl|Switch|SwitchonETimelineDirection _direction
            (:Forward
              (Variables|Default|SetIsDoorOpen true))
            (:Backward
              (Variables|Default|SetIsDoorOpen false))))))))

(event Custom|CloseDoor
  ;[1 1 1] Door opens and closes
  (if (not (Variables|Default|GetInProgress))
    (if (Variables|Default|GetIsDoorOpen)
      (bind (_direction _progressionopening) (Timeline|Timeline_0 ReverseFromEnd)
        (:Update
          (Variables|Default|SetInProgress true)
          (Transformation|SetRelativeRotation (Variables|Default|GetDoorRotator) (Math|Rotator|MakeRotator 0.0 0.0 (* (Variables|Default|GetMaxDoorOpenAngle) _progressionopening)) false false))
        (:Finished
          (Variables|Default|SetInProgress false)
          (switch Utilities|FlowControl|Switch|SwitchonETimelineDirection _direction
            (:Forward
              (Variables|Default|SetIsDoorOpen true))
            (:Backward
              (Variables|Default|SetIsDoorOpen false))))))))

(event Collision|EventActorBeginOverlap
  (params (OtherActor :type Actor%20Object%20Reference))
  ;[1 1 1] Door opens when someone is near
  (Development|PrintString "Test")
  (CallFunction|OpenDoor))

(event Collision|EventActorEndOverlap
  (params (OtherActor :type Actor%20Object%20Reference))
  ;[1 1 1] Door opens when someone is near
  (CallFunction|CloseDoor))

(fn ConstructionScript)