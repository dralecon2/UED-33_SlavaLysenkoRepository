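; BP_Toombler is a tumbler switch that toggles a door lock when flipped on or off.
; SwitchOn and SwitchOff play a timeline forward or in reverse to slide the stick mesh along local Y, guarded by the current state and an in-progress flag.
; When the timeline finishes, its direction sets the on/off state, then DoorsLockSwitch runs and a dispatcher broadcasts the new state.
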(event Custom|SwitchOn
  (if (not (Variables|Default|GetInProgress))
    (if (not (Variables|Default|GetIsTumblerOn))
      (bind (_direction _move) (Timeline|Timeline_0 PlayFromStart)
        (:Update
          (Variables|Default|SetInProgress true)
          (Transformation|SetRelativeLocation (Variables|Default|GetTumblerStickMesh) (Math|Vector|MakeVector 0.0 (* (Variables|Default|GetMaxStickOffset) _move) 0.0) false false))
        (:Finished
          (Variables|Default|SetInProgress false)
          (switch Utilities|FlowControl|Switch|SwitchonETimelineDirection _direction
            (:Forward
              (Variables|Default|SetIsTumblerOn true))
            (:Backward
              (Variables|Default|SetIsTumblerOn false)))
          (CallFunction|DoorsLockSwitch)
          (Default|CallOnDoorsLockSwitched (Variables|Default|GetIsTumblerOn)))))))

(event Custom|SwitchOff
  (if (not (Variables|Default|GetInProgress))
    (if (Variables|Default|GetIsTumblerOn)
      (bind (_direction _move) (Timeline|Timeline_0 ReverseFromEnd)
        (:Update
          (Variables|Default|SetInProgress true)
          (Transformation|SetRelativeLocation (Variables|Default|GetTumblerStickMesh) (Math|Vector|MakeVector 0.0 (* (Variables|Default|GetMaxStickOffset) _move) 0.0) false false))
        (:Finished
          (Variables|Default|SetInProgress false)
          (switch Utilities|FlowControl|Switch|SwitchonETimelineDirection _direction
            (:Forward
              (Variables|Default|SetIsTumblerOn true))
            (:Backward
              (Variables|Default|SetIsTumblerOn false)))
          (CallFunction|DoorsLockSwitch)
          (Default|CallOnDoorsLockSwitched (Variables|Default|GetIsTumblerOn)))))))

(fn ConstructionScript)